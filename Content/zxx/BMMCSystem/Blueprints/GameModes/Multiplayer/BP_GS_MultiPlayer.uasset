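; Multiplayer team-match game state that tracks two team rosters, scores, a pre-match countdown and the match timer.
; Death reports from controller server RPCs remove the actor from its team and award a point to the opposing team.
; Looping one-second timers drive countdown and match time, notifying BP_GM_Multiplayer when each ends, with winner or draw from scores.
; Countdown and match-start messages reach each player pawn's multiplayer component, while interfaces expose match status and team settings.
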(event Custom|AddToTeam
  (params (Team :type Integer) (Name :type String) (Actor :type Actor%20Object%20Reference))
  ;[1 0.8184 0 0.1] Add To Array
  (Utilities|Array|Add (Utilities|Select :Index Team :Option%200 (Variables|Teams|GetTeamANames) :Option%201 (Variables|Teams|GetTeamBNames)) Name)
  (Utilities|Array|AddUnique (Utilities|Select :Index Team :Option%200 (Variables|Teams|GetTeamAPlayers) :Option%201 (Variables|Teams|GetTeamBPlayers)) Actor))

(event Custom|ReportDeath
  (params (Actor :type Actor%20Object%20Reference))
  (bind _return (CallFunction|FGetActorTeam Actor))
  (bind _teambplayers (Variables|Teams|GetTeamBPlayers))
  (bind _teamaplayers (Variables|Teams|GetTeamAPlayers))
  (bind _returnvalue (Utilities|Select :Index _return :Option%200 _teamaplayers :Option%201 _teambplayers))
  ;[0 1 0.02679 0.1] Remove from Arrays And Update Score
  (Utilities|Array|RemoveIndex (Utilities|Select :Index _return :Option%200 (Variables|Teams|GetTeamANames) :Option%201 (Variables|Teams|GetTeamBNames)) (Utilities|Array|FindItem _returnvalue Actor))
  (Utilities|Array|RemoveItem _returnvalue Actor)
  (if (== _return 0)
    (Variables|MatchStatus|SetTeamBScore (+ (Variables|MatchStatus|GetTeamBScore) 1))
    (else
      (Variables|MatchStatus|SetTeamAScore (+ (Variables|MatchStatus|GetTeamAScore) 1)))))

(event Custom|StartCountdown
  ;[1 0.1418 0 0.1] Countdown Event
  (Variables|MatchStatus|SetCurrentCountdown 3)
  (MatchStatus|CountdownStartMessage)
  (MatchStatus|CountdownUpdateMessage)
  (bind _returnvalue (Utilities|Time|SetTimerbyEvent (delegate Custom|CountdownDecrease) 1.0 true))
  (Variables|Timers|SetCountDownTimer _returnvalue))

(event Custom|CountdownDecrease
  ;[1 0.1418 0 0.1] Countdown Event
  (bind _output_get (Variables|MatchStatus|SetCurrentCountdown (Math|Integer|Max(Integer) (- (Variables|MatchStatus|GetCurrentCountdown) 1))))
  (MatchStatus|CountdownUpdateMessage)
  (if (== _output_get 0)
    (Utilities|Time|ClearandInvalidateTimerbyHandle (Variables|Timers|GetCountDownTimer))
    (bind _asbp_gm_multiplayer (Utilities|Casting|CastToBP_GM_Multiplayer (Game|GetGameMode)))
    (Default|CountdownEnded _asbp_gm_multiplayer)))

(event Custom|StartMatchTimer
  (params (MatchTime :type Integer))
  ;[1 0.03215 0.5811 0.1] Match Timer Event
  (Variables|MatchStatus|SetMatchTime MatchTime)
  (Variables|MatchStatus|SetMatchStarted true)
  (Default|CallEDMatchStarted)
  (MatchStatus|MatchStartMessage)
  (bind _returnvalue (Utilities|Time|SetTimerbyEvent (delegate Custom|MatchTimerDecreaseEvent) 1.0 true))
  (Variables|Timers|SetMatchTimeTimer _returnvalue))

(event Custom|MatchTimerDecreaseEvent
  ;[1 0.03215 0.5811 0.1] Match Timer Event
  (bind _output_get (Variables|MatchStatus|SetMatchTime (Math|Integer|Max(Integer) (- (Variables|MatchStatus|GetMatchTime) 1))))
  (if (== _output_get 0)
    (Utilities|Time|PauseTimerbyHandle (Variables|Timers|GetMatchTimeTimer))
    (bind _asbp_gm_multiplayer (Utilities|Casting|CastToBP_GM_Multiplayer (Game|GetGameMode)))
    (Default|MatchHasEnded _asbp_gm_multiplayer (Math|Integer|SelectInt 2 (Math|Integer|SelectInt 0 1 (> (Variables|MatchStatus|GetTeamAScore) (Variables|MatchStatus|GetTeamBScore))) (== (Variables|MatchStatus|GetTeamAScore) (Variables|MatchStatus|GetTeamBScore))))
    (Variables|MatchStatus|SetMatchStarted false)
    (Variables|MatchStatus|SetMatchEnded true)
    (Default|CallEDMatchEnded)))

(fn ConstructionScript)

(fn CountdownStartMessage
  (bind _asbp_gm_multiplayer (Utilities|Casting|CastToBP_GM_Multiplayer (Game|GetGameMode)))
  (for _array_element (Variables|/Game/zxx/BMMCSystem/Blueprints/GameModes/Multiplayer/BP_GM_Multiplayer.BP_GM_Multiplayer_C|GetPlayerControllers _asbp_gm_multiplayer)
    (Class|BPLComponentsMultiplayer|IStartCountdownWidget(Message) (CallFunction|FGetMultiplayerComponent (Pawn|GetControlledPawn _array_element)))))

(fn CountdownUpdateMessage
  (bind _currentcountdown (Variables|MatchStatus|GetCurrentCountdown))
  (bind _asbp_gm_multiplayer (Utilities|Casting|CastToBP_GM_Multiplayer (Game|GetGameMode)))
  (for _array_element (Variables|/Game/zxx/BMMCSystem/Blueprints/GameModes/Multiplayer/BP_GM_Multiplayer.BP_GM_Multiplayer_C|GetPlayerControllers _asbp_gm_multiplayer)
    (Class|BPLComponentsMultiplayer|IUpdatePlayerCountdown(Message) (CallFunction|FGetMultiplayerComponent (Pawn|GetControlledPawn _array_element)) _currentcountdown (== _currentcountdown 0))))

(fn MatchStartMessage
  (bind _asbp_gm_multiplayer (Utilities|Casting|CastToBP_GM_Multiplayer (Game|GetGameMode)))
  (for _array_element (Variables|/Game/zxx/BMMCSystem/Blueprints/GameModes/Multiplayer/BP_GM_Multiplayer.BP_GM_Multiplayer_C|GetPlayerControllers _asbp_gm_multiplayer)
    (Class|BPLComponentsMultiplayer|IStartMatchWidget(Message) (CallFunction|FGetMultiplayerComponent (Pawn|GetControlledPawn _array_element)))))

(fn IGetGameModeStartDelay
  (return 0.0))

(fn IGetMatchStatus
  (return (Variables|MatchStatus|GetMatchStarted) (Variables|MatchStatus|GetMatchEnded)))

(fn IGetTeamVariables
  (return (Variables|Options|GetTeamAColor) (Variables|Options|GetTeamBColor) (Variables|Options|GetRespawnTime)))