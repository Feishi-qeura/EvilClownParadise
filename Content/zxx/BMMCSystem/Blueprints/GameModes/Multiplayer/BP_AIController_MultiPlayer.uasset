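; AI controller for multiplayer matches that activates its pawn and handles AI death and respawn.
; On possess it starts the pawn's AI immediately or on the game state's match-start event, then activates the pawn's multiplayer component after a short delay.
; Death reports go to the game state and respawn requests to the game mode through server events, while the match-info interface getters return empty defaults.
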(event Custom|PlayerDeathSERVER
  ;[1 1 1 0.1] AI Death
  (bind _asbp_gs_multi_player (Utilities|Casting|CastToBP_GS_MultiPlayer (Game|GetGameState)))
  (Default|ReportDeath _asbp_gs_multi_player (Pawn|GetControlledPawn)))

(event Custom|ActivateComp_CLIENT
  ;[1 1 1 0.1] Activate AI
  (Class|BPLComponentsMultiplayer|IMultiplayerCompActivate(Message) (CallFunction|FGetMultiplayerComponent (Pawn|GetControlledPawn))))

(event Custom|RespawnPlayerSERVER
  ;[1 1 1 0.1] AI Respawn
  (bind _asbp_gm_multiplayer (Utilities|Casting|CastToBP_GM_Multiplayer (Game|GetGameMode)))
  (Default|RespawnAIEvent _asbp_gm_multiplayer self))

(event Custom|ActivatePlayerCLIENT
  ;[1 1 1 0.1] Activate AI
  (bind _asbp_gs_multi_player (Utilities|Casting|CastToBP_GS_MultiPlayer (Game|GetGameState)))
  (if (and (Variables|/Game/zxx/BMMCSystem/Blueprints/GameModes/Multiplayer/BP_GS_MultiPlayer.BP_GS_MultiPlayer_C|GetMatchStarted _asbp_gs_multi_player) (not (Variables|/Game/zxx/BMMCSystem/Blueprints/GameModes/Multiplayer/BP_GS_MultiPlayer.BP_GS_MultiPlayer_C|GetMatchEnded _asbp_gs_multi_player)))
    (Class|BPICharacters|IAIBeginPlay(Message) (Pawn|GetControlledPawn))))

(event Custom|MatchStartEvent
  ;[1 1 1 0.1] Activate AI
  (CallFunction|ActivatePlayerCLIENT))

(event EventPossess
  (params (PossessedPawn :type Pawn%20Object%20Reference))
  ;[1 1 1 0.1] Activate AI
  (bind _asbp_gs_multi_player (Utilities|Casting|CastToBP_GS_MultiPlayer (Game|GetGameState))) ; cast is necessary here to be able to bind the event
  (if (Variables|/Game/zxx/BMMCSystem/Blueprints/GameModes/Multiplayer/BP_GS_MultiPlayer.BP_GS_MultiPlayer_C|GetMatchStarted _asbp_gs_multi_player)
    (CallFunction|ActivatePlayerCLIENT)
    (else
      (EventDispatchers|BindEventtoEDMatchStarted _asbp_gs_multi_player (delegate Custom|MatchStartEvent))))
  (Utilities|FlowControl|Delay 0.2)
  (CallFunction|ActivateCompCLIENT))

(event EventIControllerDeathReport
  ;[1 1 1 0.1] AI Death
  (if (Pawn|IsLocalController)
    (CallFunction|PlayerDeathSERVER)))

(event EventIRespawn
  ;[1 1 1 0.1] AI Respawn
  (if (Pawn|IsLocalController)
    (CallFunction|RespawnPlayerSERVER)))

(fn ConstructionScript)

(fn IGetGameModeStartDelay
  (return 0.0))

(fn IGetMatchStatus
  (return false false))

(fn IGetTeamVariables
  (return "" "" 0))