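; Networked actor whose Cube component is moved vertically by a timeline, likely as a moving platform or obstacle.
; On BeginPlay the authority starts the timeline, which adds frame-rate-scaled local Z offsets and records the resulting world position in ECPushLocation.
; Non-authority instances interpolate the cube toward ECPushLocation every tick using a non-sweeping teleport, smoothing the server-driven motion.
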(event Custom|switch
  (bind _cube (Variables|Default|GetCube))
  (bind _1 (Timeline|时间轴 PlayFromStart)
    (:Update
      (Transformation|AddLocalOffset _cube (Math|Vector|MakeVector 0.0 0.0 (* _1 (* (Utilities|Time|GetWorldDeltaSeconds) 6e+01))) false false)
      (Variables|ECAnimation|SetEC_PushLocation (Transformation|GetWorldLocation _cube)))))

(event EventBeginPlay
  (Variables|ECAnimation|SetEC_PushLocation (Transformation|GetWorldLocation (Variables|Default|GetCube)))
  (if (Ability|HasAuthority)
    (CallFunction|Switch)))

(event Collision|EventActorBeginOverlap
  (params (OtherActor :type Actor%20Object%20Reference)))

(event EventTick
  (params (DeltaSeconds :type Float%20%28single-precision%29))
  (bind _cube (Variables|Default|GetCube))
  (if (not (Ability|HasAuthority))
    (Transformation|SetWorldLocation _cube (Math|Interpolation|VInterpTo (Transformation|GetWorldLocation _cube) (Variables|ECAnimation|GetEC_PushLocation) (Utilities|Time|GetWorldDeltaSeconds) 2e+01) false true)))

(fn ConstructionScript)