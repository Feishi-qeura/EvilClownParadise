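; Player character Blueprint with hold-to-run, crouch animation notifications and a toggleable physics ragdoll, plus debug prints and a network debug widget.
; Run input switches max walk speed, and crouch events message the AnimInstance.
; Entering ragdoll detaches the simulated mesh, keeps its velocity, and runs a timer that moves the actor to the hips.
; Exiting requires slow hips, ground below and capsule clearance before reattaching the mesh and resuming in Falling.
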(event Input|EnhancedActionEvents|EnhancedInputActionIAC_Run
  (params (ActionValue :type Boolean) (ElapsedSeconds :type Float%20%28double-precision%29) (TriggeredSeconds :type Float%20%28double-precision%29) (InputAction :type Input%20Action%20Object%20Reference :default "/Game/_Game/Animations/IAC_Run.IAC_Run"))
  (:Started
    (CallFunction|ECSetRunning true))
  (:Canceled
    (CallFunction|ECSetRunning false :!label _label))
  (:Completed
    (goto _label)))

(event Input|EnhancedActionEvents|EnhancedInputActionIAC_Ragdoll
  (params (ActionValue :type Boolean) (ElapsedSeconds :type Float%20%28double-precision%29) (TriggeredSeconds :type Float%20%28double-precision%29) (InputAction :type Input%20Action%20Object%20Reference :default "/Game/_Game/Animations/IAC_Ragdoll.IAC_Ragdoll"))
  (:Started
    (CallFunction|ECToggleRagdoll)))

(event EventBeginPlay
  (Variables|ECAnimation|SetEC_MeshRelative (Transformation|GetRelativeTransform (Variables|Character|GetMesh)))
  (Variables|ECAnimation|SetEC_StandingHalfHeight (Components|Capsule|GetScaledCapsuleHalfHeight (Variables|Default|GetCapsuleComponent)))
  (bind _returnvalue (UserInterface|CreateWidget "/Game/zxx/Widget/BP_NetworkDebug.BP_NetworkDebug_C"))
  (UserInterface|Viewport|AddtoViewport _returnvalue 0)
  (bind _pingvalue (|FUCheckSessionStatus 1.0)
    (:OnServer
      (Development|PrintString (Utilities|String|Append "server :" (Utilities|String|ToString(Float) _pingvalue))))
    (:OnClient
      (Development|PrintString (Utilities|String|Append "Client :" (Utilities|String|ToString(Float) _pingvalue))))))

(event Collision|EventActorBeginOverlap
  (params (OtherActor :type Actor%20Object%20Reference)))

(event EventTick
  (params (DeltaSeconds :type Float%20%28single-precision%29)))

(event EventOnStartCrouch
  (params (HalfHeightAdjust :type Float%20%28single-precision%29) (ScaledHalfHeightAdjust :type Float%20%28single-precision%29))
  (Class|BPIAnimationEvent|EventAnimationCrouch(Message) (Components|SkeletalMesh|GetAnimInstance (Variables|Character|GetMesh)) true))

(event EventOnEndCrouch
  (params (HalfHeightAdjust :type Float%20%28single-precision%29) (ScaledHalfHeightAdjust :type Float%20%28single-precision%29))
  (Class|BPIAnimationEvent|EventAnimationCrouch(Message) (Components|SkeletalMesh|GetAnimInstance (Variables|Character|GetMesh)) false))

(event EventOnJumped
  (Development|PrintString "Hello"))

(event EventOnLanded
  (params (Hit :type Hit%20Result%20Structure%20%28by%20ref%29))
  (Development|PrintString "Hello"))

(fn ConstructionScript)

(fn ECSetRunning
  (params (Running :type Boolean))
  (bind _charactermovement (Variables|Character|GetCharacterMovement))
  (Variables|ECAnimation|SetEC_RunHeld Running)
  (if Running
    (Variables|/Script/Engine.CharacterMovementComponent|SetMaxWalkSpeed _charactermovement 4.5e+02)
    (else
      (Variables|/Script/Engine.CharacterMovementComponent|SetMaxWalkSpeed _charactermovement 1.8e+02))))

(fn ECToggleRagdoll
  (if (not (Class|ECPCharBase|IsDead))
    (if (Variables|ECAnimation|GetEC_Ragdoll)
      (CallFunction|ECExitRagdoll)
      (else
        (CallFunction|ECEnterRagdoll)))))

(fn ECEnterRagdoll
  (bind _mesh (Variables|Character|GetMesh))
  (bind _charactermovement (Variables|Character|GetCharacterMovement))
  (if (not (Variables|ECAnimation|GetEC_Ragdoll))
    (Variables|ECAnimation|SetEC_EntryVelocity (Transformation|GetVelocity))
    (Character|StopJumping)
    (Character|UnCrouch)
    (Variables|ECAnimation|SetEC_Ragdoll true)
    (Components|Movement|StopMovementImmediately _charactermovement)
    (Pawn|Components|CharacterMovement|DisableMovement _charactermovement)
    (Collision|SetCollisionEnabled (Variables|Default|GetCapsuleComponent) "NoCollision")
    (Transformation|DetachFromComponent _mesh "KeepWorld" "KeepWorld" "KeepWorld" true)
    (Collision|SetCollisionProfileName _mesh "Ragdoll" true :!class /Script/Engine.PrimitiveComponent)
    (Physics|SetSimulatePhysics _mesh true)
    (Class|SkeletalMeshComponent|SetPhysicsBlendWeight _mesh 1.0)
    (Class|PrimitiveComponent|SetAllPhysicsLinearVelocity _mesh (Variables|ECAnimation|GetEC_EntryVelocity) false)
    (Class|PrimitiveComponent|WakeAllRigidBodies _mesh)
    (Utilities|Time|SetTimerbyFunctionName 0 "EC_UpdateRagdoll" 0.016667 true true)))

(fn ECExitRagdoll
  (bind _mesh (Variables|Character|GetMesh))
  (bind _capsulecomponent (Variables|Default|GetCapsuleComponent))
  (bind _ec_standinghalfheight (Variables|ECAnimation|GetEC_StandingHalfHeight))
  (bind _returnvalue (Transformation|GetSocketLocation _mesh "Hips"))
  (if (Variables|ECAnimation|GetEC_Ragdoll)
    (bind _returnvalue_2 (Physics|GetPhysicsLinearVelocity _mesh "Hips"))
    (if (< (Math|Vector|VectorLength _returnvalue_2) 1.6e+02)
      (bind (_outhit _returnvalue_3) (Collision|LineTraceByChannel (+ _returnvalue "0,0,50") (+ _returnvalue "0,0,-160") "TraceTypeQuery1" false 0 "None"))
      (if _returnvalue_3
        (bind _returnvalue_4 (Class|KismetSystemLibrary|CapsuleTraceSinglebyProfile (+ (.ImpactPoint (Collision|BreakHitResult _outhit)) (Math|Vector|MakeVector 0.0 0.0 (+ _ec_standinghalfheight 4.0))) (+ (.ImpactPoint (Collision|BreakHitResult _outhit)) (Math|Vector|MakeVector 0.0 0.0 (+ _ec_standinghalfheight 4.0))) (Components|Capsule|GetScaledCapsuleRadius _capsulecomponent) _ec_standinghalfheight "Pawn" false 0 "None" true))
        (if (not _returnvalue_4)
          (Physics|SetSimulatePhysics _mesh false)
          (Class|SkeletalMeshComponent|SetPhysicsBlendWeight _mesh 0.0)
          (Transformation|SetActorLocation (+ (.ImpactPoint (Collision|BreakHitResult _outhit)) (Math|Vector|MakeVector 0.0 0.0 (+ _ec_standinghalfheight 4.0))) false true)
          (Transformation|AttachComponentToComponent _mesh _capsulecomponent "None" "KeepRelative" "KeepRelative" "KeepRelative" false)
          (Transformation|SetRelativeTransform _mesh (Variables|ECAnimation|GetEC_MeshRelative) false true)
          (Collision|SetCollisionProfileName _mesh "CharacterMesh" true :!class /Script/Engine.PrimitiveComponent)
          (Collision|SetCollisionEnabled _capsulecomponent "QueryAndPhysics")
          (Character|StopJumping)
          (Character|UnCrouch)
          (Pawn|Components|CharacterMovement|SetMovementMode (Variables|Character|GetCharacterMovement) "MOVE_Falling" 0)
          (Variables|ECAnimation|SetEC_Ragdoll false)
          (Utilities|Time|ClearTimerbyFunctionName 0 "EC_UpdateRagdoll"))))))

(fn ECUpdateRagdoll
  (if (Variables|ECAnimation|GetEC_Ragdoll)
    (Transformation|SetActorLocation (Transformation|GetSocketLocation (Variables|Character|GetMesh) "Hips") false true)))