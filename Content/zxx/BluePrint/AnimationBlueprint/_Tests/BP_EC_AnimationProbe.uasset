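; Test probe actor that drives the BP_ECPlayer character with simulated input and records the resulting movement and animation state.
; Each Tick it injects its input variables into the Enhanced Input move, jump, crouch, run and ragdoll actions on player 0.
; It then copies the character's speed, direction, location, air, crouch and ragdoll state, plus AMT_Jump montage playback and section, into Observed variables.
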(event EventBeginPlay)

(event Collision|EventActorBeginOverlap
  (params (OtherActor :type Actor%20Object%20Reference)))

(event EventTick
  (params (DeltaSeconds :type Float%20%28single-precision%29))
  (bind _returnvalue (Game|GetPlayerController 0))
  (bind _returnvalue_2 (PlayerController|LocalPlayerSubsystems|GetEnhancedInputLocalPlayerSubsystem _returnvalue))
  (Class|EnhancedInputSubsystemInterface|InjectInputVectorforAction _returnvalue_2 "/Game/zxx/Input/Action/IAC_Move.IAC_Move" (Variables|ECAnimation|GetMoveInput))
  (Class|EnhancedInputSubsystemInterface|InjectInputVectorforAction _returnvalue_2 "/Game/zxx/Input/Action/IAC_Jump.IAC_Jump" (Variables|ECAnimation|GetJumpInput))
  (Class|EnhancedInputSubsystemInterface|InjectInputVectorforAction _returnvalue_2 "/Game/zxx/Input/Action/IAC_SquatDown.IAC_SquatDown" (Variables|ECAnimation|GetCrouchInput))
  (Class|EnhancedInputSubsystemInterface|InjectInputVectorforAction _returnvalue_2 "/Game/zxx/BluePrint/AnimationBlueprint/IAC_Run.IAC_Run" (Variables|ECAnimation|GetRunInput))
  (Class|EnhancedInputSubsystemInterface|InjectInputVectorforAction _returnvalue_2 "/Game/zxx/BluePrint/AnimationBlueprint/IAC_Ragdoll.IAC_Ragdoll" (Variables|ECAnimation|GetRagdollInput))
  (bind _asbp_ecplayer (Utilities|Casting|CastToBP_ECPlayer (Game|GetPlayerCharacter 0)))
  (Variables|ECAnimation|SetObservedSpeed (Math|Vector|VectorLengthXY (Transformation|GetVelocity _asbp_ecplayer)))
  (Variables|ECAnimation|SetObservedDirection (Class|KismetAnimationLibrary|CalculateDirection (Transformation|GetVelocity _asbp_ecplayer) (Transformation|GetActorRotation _asbp_ecplayer)))
  (Variables|ECAnimation|SetObservedInAir (AI|Components|NavMovement|IsFalling (Variables|/Script/Engine.Character|GetCharacterMovement _asbp_ecplayer)))
  (Variables|ECAnimation|SetObservedCrouched (Variables|/Script/Engine.Character|GetbIsCrouched _asbp_ecplayer))
  (Variables|ECAnimation|SetObservedLocation (Transformation|GetActorLocation _asbp_ecplayer))
  (Variables|ECAnimation|SetObservedRagdoll (Variables|/Game/zxx/BluePrint/Player/BP_ECPlayer.BP_ECPlayer_C|GetEC_Ragdoll _asbp_ecplayer))
  (if (Utilities|IsValid (Components|SkeletalMesh|GetAnimInstance (Variables|/Script/Engine.Character|GetMesh _asbp_ecplayer)))
    (Variables|ECAnimation|SetObservedJumpSection (Animation|Montage|MontageGetCurrentSection (Components|SkeletalMesh|GetAnimInstance (Variables|/Script/Engine.Character|GetMesh _asbp_ecplayer)) "/Game/zxx/BluePrint/AnimationBlueprint/AMT_Jump.AMT_Jump"))
    (Variables|ECAnimation|SetObservedJumpMontagePlaying (Animation|Montage|MontageIsPlaying (Components|SkeletalMesh|GetAnimInstance (Variables|/Script/Engine.Character|GetMesh _asbp_ecplayer)) "/Game/zxx/BluePrint/AnimationBlueprint/AMT_Jump.AMT_Jump"))
    (else
      (Variables|ECAnimation|SetObservedJumpSection "None")
      (Variables|ECAnimation|SetObservedJumpMontagePlaying false))))

(fn ConstructionScript)