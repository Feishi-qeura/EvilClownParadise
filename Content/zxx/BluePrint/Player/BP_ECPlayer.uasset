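; Player character with replicated running, crouch animation messages, and a server-authoritative ragdoll toggle.
; The server simulates ragdoll physics and sends 20 Hz pose snapshots in a fixed reference frame, which clients accept without simulating.
; A sequenced RepNotify struct drives ragdoll, stand-up and jump-landing phases.
; Stand-up requires slow hips and clear ground; both landing phases lock movement until the montage ends and the owner confirms.
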(event Custom|EC_ServerToggleRagdoll
  (bind _ec_netragdollstate (Variables|Default|GetEC_NetRagdollState))
  (bind (_phase _sequence _anchorlocation _entryvelocity _recoverytransform) (Utilities|Struct|BreakST_EC_RagdollNetState _ec_netragdollstate))
  (if (Ability|HasAuthority)
    (if (not (or (== _phase 2) (== _phase 3)))
      (CallFunction|ECToggleRagdoll))))

(event Custom|EC_ServerRecoveryReady
  (bind _ec_netragdollstate (Variables|Default|GetEC_NetRagdollState))
  (bind (_phase _sequence _anchorlocation _entryvelocity _recoverytransform) (Utilities|Struct|BreakST_EC_RagdollNetState _ec_netragdollstate))
  (if (Ability|HasAuthority)
    (if (or (== _phase 2) (== _phase 3))
      (Variables|ECAnimation|SetEC_RecoveryOwnerReady true)
      (CallFunction|ECTryFinishRecovery))))

(event Custom|EC_ServerStartRunning
  (if (Ability|HasAuthority)
    (CallFunction|ECSetRunning true)))

(event Custom|EC_ServerStopRunning
  (if (Ability|HasAuthority)
    (CallFunction|ECSetRunning false)))

(event Input|EnhancedActionEvents|EnhancedInputActionIAC_Run
  (params (ActionValue :type Boolean) (ElapsedSeconds :type Float%20%28double-precision%29) (TriggeredSeconds :type Float%20%28double-precision%29) (InputAction :type Input%20Action%20Object%20Reference :default "/Game/_Game/Animations/IAC_Run.IAC_Run"))
  (:Started
    (CallFunction|ECSetRunning true))
  (:Canceled
    (CallFunction|ECSetRunning false :!label _label))
  (:Completed
    (goto _label)))

(event Input|EnhancedActionEvents|EnhancedInputActionIAC_Ragdoll
  (params (ActionValue :type Boolean) (ElapsedSeconds :type Float%20%28double-precision%29) (TriggeredSeconds :type Float%20%28double-precision%29) (InputAction :type Input%20Action%20Object%20Reference :default "/Game/_Game/Animations/IAC_Ragdoll.IAC_Ragdoll"))
  (:Started
    (CallFunction|ECServerToggleRagdoll)))

(event EventBeginPlay
  (Variables|ECAnimation|SetEC_MeshRelative (Transformation|GetRelativeTransform (Variables|Character|GetMesh)))
  (Variables|ECAnimation|SetEC_StandingHalfHeight (Components|Capsule|GetScaledCapsuleHalfHeight (Variables|Default|GetCapsuleComponent)))
  (bind _returnvalue (UserInterface|CreateWidget "/Game/zxx/Widget/BP_NetworkDebug.BP_NetworkDebug_C"))
  (UserInterface|Viewport|AddtoViewport _returnvalue 0)
  (bind _pingvalue (|FUCheckSessionStatus 1.0)
    (:OnServer
      (Development|PrintString (Utilities|String|Append "server :" (Utilities|String|ToString(Float) _pingvalue))))
    (:OnClient
      (Development|PrintString (Utilities|String|Append "Client :" (Utilities|String|ToString(Float) _pingvalue))))))

(event Collision|EventActorBeginOverlap
  (params (OtherActor :type Actor%20Object%20Reference)))

(event EventTick
  (params (DeltaSeconds :type Float%20%28single-precision%29))
  (CallFunction|ECTickRagdollPose))

(event EventOnStartCrouch
  (params (HalfHeightAdjust :type Float%20%28single-precision%29) (ScaledHalfHeightAdjust :type Float%20%28single-precision%29))
  (Class|BPIAnimationEvent|EventAnimationCrouch(Message) (Components|SkeletalMesh|GetAnimInstance (Variables|Character|GetMesh)) true))

(event EventOnEndCrouch
  (params (HalfHeightAdjust :type Float%20%28single-precision%29) (ScaledHalfHeightAdjust :type Float%20%28single-precision%29))
  (Class|BPIAnimationEvent|EventAnimationCrouch(Message) (Components|SkeletalMesh|GetAnimInstance (Variables|Character|GetMesh)) false))

(event EventOnJumped
  (Development|PrintString "Hello"))

(event EventOnLanded
  (params (Hit :type Hit%20Result%20Structure%20%28by%20ref%29))
  (Development|PrintString "Hello")
  (CallFunction|ECHandleLanded))

(fn ConstructionScript)

(fn ECSetRunning
  (params (Running :type Boolean))
  (Variables|ECAnimation|SetEC_RunHeld Running)
  (CallFunction|ECRequestRunState))

(fn ECToggleRagdoll
  (if (Ability|HasAuthority)
    (if (not (Class|ECPCharBase|IsDead))
      (if (Variables|ECAnimation|GetEC_Ragdoll)
        (CallFunction|ECExitRagdoll)
        (else
          (CallFunction|ECEnterRagdoll))))))

(fn ECEnterRagdoll
  (bind _returnvalue (Ability|HasAuthority))
  (bind _mesh (Variables|Character|GetMesh))
  (bind _charactermovement (Variables|Character|GetCharacterMovement))
  (if (not (Variables|ECAnimation|GetEC_Ragdoll))
    ;[0.15 0.15 0.15 0.5] 【2026-09-18同步修订】保留原输入锁与移动隔离
    ; Detach后先EC_InitPoseFrame；HasAuthority=true才进入Ragdoll碰撞/模拟/初速度/20Hz计时器。
    ; 客户端跳过上述物理链，只接收姿态。Phase1.RecoveryTransform在此阶段承载固定姿态参考坐标系。
    ; 服务器先发布新序号Phase1，再采样首个快照。起身Phase2仍使用真正的站立RecoveryTransform。
    (Utilities|Time|ClearTimerbyFunctionName 0 "EC_PollRecoveryLanding")
    (Variables|ECAnimation|SetEC_NormalLanding false)
    (if (Variables|ECAnimation|GetEC_InputLocked)
      _
      (else
        (Variables|ECAnimation|SetEC_PreTickEnabled (Class|ActorComponent|IsComponentTickEnabled _charactermovement))
        (Variables|ECAnimation|SetEC_PreIgnoreClientCorrections (Variables|/Script/Engine.CharacterMovementComponent|GetbClientIgnoreMovementCorrections _charactermovement))
        (Variables|ECAnimation|SetEC_PreIgnoreServerCorrections (Variables|/Script/Engine.CharacterMovementComponent|GetbIgnoreClientMovementErrorChecksAndCorrection _charactermovement))
        (Variables|ECAnimation|SetEC_InputLocked true)
        (Variables|/Script/Engine.CharacterMovementComponent|SetbClientIgnoreMovementCorrections _charactermovement true)
        (Variables|/Script/Engine.CharacterMovementComponent|SetbIgnoreClientMovementErrorChecksAndCorrection _charactermovement true)
        (if (Pawn|IsLocallyControlled)
          (Input|SetIgnoreMoveInput (Pawn|GetController) true))))
    (Class|Pawn|ConsumeMovementInputVector)
    (Variables|ECAnimation|SetEC_EntryVelocity (Math|Vector|SelectVector (Transformation|GetVelocity) (.EntryVelocity (Utilities|Struct|BreakST_EC_RagdollNetState (Variables|Default|GetEC_NetRagdollState))) (Ability|HasAuthority)))
    (Character|StopJumping)
    (Character|UnCrouch)
    (Variables|ECAnimation|SetEC_Ragdoll true)
    (Components|Movement|StopMovementImmediately _charactermovement)
    (Pawn|Components|CharacterMovement|DisableMovement _charactermovement)
    (Components|Tick|SetComponentTickEnabled _charactermovement false)
    (Class|Actor|SetReplicateMovement false)
    (Collision|SetCollisionEnabled (Variables|Default|GetCapsuleComponent) "NoCollision")
    (Transformation|DetachFromComponent _mesh "KeepWorld" "KeepWorld" "KeepWorld" true)
    (CallFunction|ECInitPoseFrame)
    (if _returnvalue
      (Collision|SetCollisionProfileName _mesh "Ragdoll" true :!class /Script/Engine.PrimitiveComponent)
      (Physics|SetSimulatePhysics _mesh true)
      (Class|SkeletalMeshComponent|SetPhysicsBlendWeight _mesh 1.0)
      (Class|PrimitiveComponent|SetAllPhysicsLinearVelocity _mesh (Variables|ECAnimation|GetEC_EntryVelocity) false)
      (Class|PrimitiveComponent|WakeAllRigidBodies _mesh)
      (Utilities|Time|SetTimerbyFunctionName 0 "EC_UpdateRagdoll" 0.05 true true)
      (if _returnvalue
        (CallFunction|ECPublishRagdollState 1 (Transformation|GetSocketLocation _mesh "Hips") (Variables|ECAnimation|GetEC_EntryVelocity) (Variables|Default|GetEC_PoseFrame) true)
        (CallFunction|ECCaptureNetPose))
      (else
        (CallFunction|ECAcceptNetPose)))))

(fn ECExitRagdoll
  (bind _mesh (Variables|Character|GetMesh))
  (bind _ec_standinghalfheight (Variables|ECAnimation|GetEC_StandingHalfHeight))
  (bind _returnvalue (Transformation|GetSocketLocation _mesh "Hips"))
  (if (Ability|HasAuthority)
    (if (Variables|ECAnimation|GetEC_Ragdoll)
      (bind _returnvalue_2 (Physics|GetPhysicsLinearVelocity _mesh "Hips"))
      (if (< (Math|Vector|VectorLength _returnvalue_2) 1.6e+02)
        (bind (_outhit _returnvalue_3) (Collision|LineTraceByChannel (+ _returnvalue "0,0,50") (+ _returnvalue "0,0,-160") "TraceTypeQuery1" false 0 "ForDuration"))
        (if _returnvalue_3
          (bind _returnvalue_4 (Class|KismetSystemLibrary|CapsuleTraceSinglebyProfile (+ (.ImpactPoint (Collision|BreakHitResult _outhit)) (Math|Vector|MakeVector 0.0 0.0 (+ _ec_standinghalfheight 4.0))) (+ (.ImpactPoint (Collision|BreakHitResult _outhit)) (Math|Vector|MakeVector 0.0 0.0 (+ _ec_standinghalfheight 4.0))) (Components|Capsule|GetScaledCapsuleRadius (Variables|Default|GetCapsuleComponent)) _ec_standinghalfheight "Pawn" false 0 "ForDuration" true))
          (if (not _returnvalue_4)
            (CallFunction|ECPublishRagdollState 2 _returnvalue "0, 0, 0" (Math|Transform|MakeTransform (+ (.ImpactPoint (Collision|BreakHitResult _outhit)) (Math|Vector|MakeVector 0.0 0.0 (+ _ec_standinghalfheight 4.0))) (Transformation|GetActorRotation)) true)))))))

(fn ECUpdateRagdoll
  (bind _mesh (Variables|Character|GetMesh))
  (if (Variables|ECAnimation|GetEC_Ragdoll)
    (if (Ability|HasAuthority)
      (bind _returnvalue (Physics|GetPhysicsLinearVelocity _mesh "Hips"))
      (CallFunction|ECPublishRagdollState 1 (Transformation|GetSocketLocation _mesh "Hips") _returnvalue (.RecoveryTransform (Utilities|Struct|BreakST_EC_RagdollNetState (Variables|Default|GetEC_NetRagdollState))) false)
      (CallFunction|ECCaptureNetPose))))

(fn ECApplyNetRagdoll
  (bind _ec_netragdollstate (Variables|Default|GetEC_NetRagdollState))
  (bind (_phase _sequence _anchorlocation _entryvelocity _recoverytransform) (Utilities|Struct|BreakST_EC_RagdollNetState _ec_netragdollstate))
  (if (not (== _sequence (Variables|ECAnimation|GetEC_LastAppliedSequence)))
    (Variables|ECAnimation|SetEC_LastAppliedSequence _sequence)
    (if (== _phase 1)
      (CallFunction|ECEnterRagdoll)
      (elif (== _phase 2)
        (CallFunction|ECEnterRagdoll)
        (CallFunction|ECApplyRecovery _recoverytransform)
        (CallFunction|ECStartRecoveryLanding)
        (elif (== _phase 3)
          (CallFunction|ECBeginJumpLanding)
          (Transformation|SetActorTransform _recoverytransform false true)
          (Components|Tick|SetComponentTickEnabled (Variables|Character|GetCharacterMovement) (Variables|ECAnimation|GetEC_PreTickEnabled))
          (Class|Actor|SetReplicateMovement true)
          (else
            (CallFunction|ECApplyRecovery _recoverytransform)
            (CallFunction|ECFinishRecovery)))))))

(fn ECApplyRecovery
  (params (RecoveryTransform :type Transform))
  (bind _mesh (Variables|Character|GetMesh))
  (bind _capsulecomponent (Variables|Default|GetCapsuleComponent))
  (if (Variables|ECAnimation|GetEC_Ragdoll)
    (Utilities|Time|ClearTimerbyFunctionName 0 "EC_UpdateRagdoll")
    (Physics|SetSimulatePhysics _mesh false)
    (Class|SkeletalMeshComponent|SetPhysicsBlendWeight _mesh 0.0)
    (Transformation|SetActorTransform RecoveryTransform false true)
    (Transformation|AttachComponentToComponent _mesh _capsulecomponent "None" "KeepRelative" "KeepRelative" "KeepRelative" false)
    (Transformation|SetRelativeTransform _mesh (Variables|ECAnimation|GetEC_MeshRelative) false true)
    (Collision|SetCollisionProfileName _mesh "CharacterMesh" true :!class /Script/Engine.PrimitiveComponent)
    (Collision|SetCollisionEnabled _capsulecomponent "QueryAndPhysics")
    (Character|StopJumping)
    (Character|UnCrouch)
    (Variables|ECAnimation|SetEC_Ragdoll false)
    (Class|ActorComponent|SetIsReplicated _mesh (Variables|ECAnimation|GetEC_PreMeshReplicated))
    (Variables|/Script/Engine.SkinnedMeshComponent|SetVisibilityBasedAnimTickOption _mesh (Utilities|Enum|ByteToEnumEVisibilityBasedAnimTickOption (Variables|ECAnimation|GetEC_PrePoseTickMode)))))

(fn ECFinishRecovery
  (bind _charactermovement (Variables|Character|GetCharacterMovement))
  (if (Variables|ECAnimation|GetEC_InputLocked)
    (Variables|/Script/Engine.CharacterMovementComponent|SetbClientIgnoreMovementCorrections _charactermovement (Variables|ECAnimation|GetEC_PreIgnoreClientCorrections))
    (Variables|/Script/Engine.CharacterMovementComponent|SetbIgnoreClientMovementErrorChecksAndCorrection _charactermovement (Variables|ECAnimation|GetEC_PreIgnoreServerCorrections))
    (Components|Tick|SetComponentTickEnabled _charactermovement (Variables|ECAnimation|GetEC_PreTickEnabled))
    (Class|Actor|SetReplicateMovement true)
    (Pawn|Components|CharacterMovement|SetMovementMode _charactermovement "MOVE_Walking" 0)
    (Class|Pawn|ConsumeMovementInputVector)
    (Character|StopJumping)
    (if (Pawn|IsLocallyControlled)
      (Input|SetIgnoreMoveInput (Pawn|GetController) false))
    (Variables|ECAnimation|SetEC_InputLocked false)
    (Variables|ECAnimation|SetEC_NormalLanding false)))

(fn ECPublishRagdollState
  (params (Phase :type Integer) (AnchorLocation :type Vector) (EntryVelocity :type Vector) (RecoveryTransform :type Transform) (AdvanceSequence :type Boolean))
  (if (Ability|HasAuthority)
    (if AdvanceSequence
      (Variables|ECAnimation|SetEC_NetSequence (+ (Variables|ECAnimation|GetEC_NetSequence) 1)))
    (Variables|Default|SetEC_NetRagdollState (Utilities|Struct|MakeST_EC_RagdollNetState Phase (Variables|ECAnimation|GetEC_NetSequence) AnchorLocation EntryVelocity RecoveryTransform))
    (if AdvanceSequence
      (Networking|ForceNetUpdate))))

(fn OnRepECNetRagdollState
  ;[0.15 0.15 0.15 0.5] 持久网络状态入口
  ; Phase、Sequence、锚点、速度、恢复位置放在同一个 RepNotify 结构体。
  ; 避免先收到起身状态、后收到起身位置；新进入相关范围的客户端也能取得当前状态。
  (CallFunction|ECApplyNetRagdoll))

(fn ECStartRecoveryLanding
  (bind _mesh (Variables|Character|GetMesh))
  (bind _returnvalue (Components|SkeletalMesh|GetAnimInstance _mesh))
  (Variables|ECAnimation|SetEC_RecoveryAnimationDone false)
  (Variables|ECAnimation|SetEC_RecoveryOwnerReady false)
  (Animation|Montage|MontagePlay _returnvalue "/Game/_Game/Animations/Montage/AMT_Jump.AMT_Jump" 1.0 "MontageLength" 0.0 true)
  (Ability|Animation|MontageJumptoSection _returnvalue "Landing" "/Game/_Game/Animations/Montage/AMT_Jump.AMT_Jump")
  (Class|AnimInstance|MontageSetNextSection _returnvalue "Landing" "None" "/Game/_Game/Animations/Montage/AMT_Jump.AMT_Jump")
  (Utilities|Time|SetTimerbyFunctionName 0 "EC_PollRecoveryLanding" 0.03 true true))

(fn ECPollRecoveryLanding
  (bind _ec_netragdollstate (Variables|Default|GetEC_NetRagdollState))
  (bind _phase (Utilities|Struct|BreakST_EC_RagdollNetState _ec_netragdollstate))
  (if (or (== _phase 2) (== _phase 3))
    (if (not (Class|AnimInstance|IsAnyMontagePlaying (Components|SkeletalMesh|GetAnimInstance (Variables|Character|GetMesh))))
      (Utilities|Time|ClearTimerbyFunctionName 0 "EC_PollRecoveryLanding")
      (Variables|ECAnimation|SetEC_RecoveryAnimationDone true)
      (if (Pawn|IsLocallyControlled)
        (CallFunction|ECServerRecoveryReady)
        (else
          (CallFunction|ECTryFinishRecovery))))
    (elif (not (Variables|ECAnimation|GetEC_NormalLanding))
      (Utilities|Time|ClearTimerbyFunctionName 0 "EC_PollRecoveryLanding"))))

(fn ECTryFinishRecovery
  (bind _ec_netragdollstate (Variables|Default|GetEC_NetRagdollState))
  (bind (_phase _sequence _anchorlocation _entryvelocity _recoverytransform) (Utilities|Struct|BreakST_EC_RagdollNetState _ec_netragdollstate))
  (if (Ability|HasAuthority)
    (if (or (== _phase 2) (== _phase 3))
      (if (Variables|ECAnimation|GetEC_RecoveryAnimationDone)
        (if (Variables|ECAnimation|GetEC_RecoveryOwnerReady)
          (CallFunction|ECPublishRagdollState 0 _anchorlocation _entryvelocity _recoverytransform true))))))

(fn ECBeginJumpLanding
  (bind _charactermovement (Variables|Character|GetCharacterMovement))
  (if (not (Variables|ECAnimation|GetEC_InputLocked))
    (Variables|ECAnimation|SetEC_PreTickEnabled (Class|ActorComponent|IsComponentTickEnabled _charactermovement))
    (Variables|ECAnimation|SetEC_PreIgnoreClientCorrections (Variables|/Script/Engine.CharacterMovementComponent|GetbClientIgnoreMovementCorrections _charactermovement))
    (Variables|ECAnimation|SetEC_PreIgnoreServerCorrections (Variables|/Script/Engine.CharacterMovementComponent|GetbIgnoreClientMovementErrorChecksAndCorrection _charactermovement))
    (Variables|ECAnimation|SetEC_NormalLanding true)
    (Variables|ECAnimation|SetEC_InputLocked true)
    (Variables|/Script/Engine.CharacterMovementComponent|SetbClientIgnoreMovementCorrections _charactermovement true)
    (Variables|/Script/Engine.CharacterMovementComponent|SetbIgnoreClientMovementErrorChecksAndCorrection _charactermovement true)
    (Character|StopJumping)
    (Components|Movement|StopMovementImmediately _charactermovement)
    (Pawn|Components|CharacterMovement|DisableMovement _charactermovement)
    (if (Pawn|IsLocallyControlled)
      (Input|SetIgnoreMoveInput (Pawn|GetController) true))
    (Class|Pawn|ConsumeMovementInputVector)
    (CallFunction|ECStartRecoveryLanding)))

(fn ECHandleLanded
  (if (not (Variables|ECAnimation|GetEC_InputLocked))
    (if (Ability|HasAuthority)
      (CallFunction|ECPublishRagdollState 3 (Transformation|GetActorLocation) "0, 0, 0" (Transformation|GetActorTransform) true)
      (else
        (CallFunction|ECBeginJumpLanding)))))

(fn OnRepECRunHeld
  (bind _charactermovement (Variables|Character|GetCharacterMovement))
  (if (Variables|ECAnimation|GetEC_RunHeld)
    (Variables|/Script/Engine.CharacterMovementComponent|SetMaxWalkSpeed _charactermovement 4.5e+02)
    (else
      (Variables|/Script/Engine.CharacterMovementComponent|SetMaxWalkSpeed _charactermovement 1.8e+02))))

(fn ECRequestRunState
  (if (not (Ability|HasAuthority))
    (if (Pawn|IsLocallyControlled)
      (if (Variables|ECAnimation|GetEC_RunHeld)
        (CallFunction|ECServerStartRunning)
        (else
          (CallFunction|ECServerStopRunning))))))

(fn OnRepECNetPose
  (CallFunction|ECAcceptNetPose))

(fn ECCaptureNetPose
  (bind _mesh (Variables|Character|GetMesh))
  (bind _ec_capturedpose (Variables|Default|GetEC_CapturedPose))
  (bind (_localtransforms _bonenames _skeletalmeshname _snapshotname _bisvalid) (Utilities|Struct|BreakPoseSnapshot _ec_capturedpose))
  (Class|SkeletalMeshComponent|SnapshotPose _mesh _ec_capturedpose)
  (Variables|Default|SetEC_CaptureTransforms _localtransforms)
  (Utilities|Array|SetArrayElem (Variables|Default|GetEC_CaptureTransforms) 0 (Math|Transform|MakeRelativeTransform (Math|Transform|ComposeTransforms (Utilities|Array|Get(acopy) (Variables|Default|GetEC_CaptureTransforms)) (Transformation|GetWorldTransform _mesh)) (Variables|Default|GetEC_PoseFrame)))
  (Variables|Default|SetEC_NetPose (Utilities|Struct|MakePoseSnapshot (Variables|Default|GetEC_CaptureTransforms) _bonenames _skeletalmeshname (Utilities|String|StringToName (Utilities|String|ToString(Integer) (Variables|ECAnimation|GetEC_NetSequence))) _bisvalid))
  (Networking|ForceNetUpdate))

(fn ECAcceptNetPose
  (bind _ec_netpose (Variables|Default|GetEC_NetPose))
  (bind (_localtransforms _bonenames _skeletalmeshname _snapshotname _bisvalid) (Utilities|Struct|BreakPoseSnapshot _ec_netpose))
  (if (not (Ability|HasAuthority))
    (if (Variables|ECAnimation|GetEC_Ragdoll)
      (if _bisvalid
        (if (== (Utilities|String|StringToName (Utilities|String|ToString(Integer) (.Sequence (Utilities|Struct|BreakST_EC_RagdollNetState (Variables|Default|GetEC_NetRagdollState))))) _snapshotname)
          (if (Variables|ECAnimation|GetEC_PoseReady)
            (Class|SkeletalMeshComponent|SnapshotPose (Variables|Character|GetMesh) (Variables|Default|GetEC_PosePrevious))
            (else
              (Variables|Default|SetEC_PosePrevious _ec_netpose)))
          (Variables|Default|SetEC_PoseTarget _ec_netpose)
          (Variables|ECAnimation|SetEC_PoseBlend 0.0)
          (Variables|ECAnimation|SetEC_PoseReady true))))))

(fn ECTickRagdollPose
  (if (Variables|ECAnimation|GetEC_Ragdoll)
    (if (Ability|HasAuthority)
      (Transformation|SetActorLocation (Transformation|GetSocketLocation (Variables|Character|GetMesh) "Hips") false true :!label _label)
      (elif (Variables|ECAnimation|GetEC_PoseReady)
        (goto _label)))))

(fn ECInitPoseFrame
  (bind _mesh (Variables|Character|GetMesh))
  (Variables|ECAnimation|SetEC_PrePoseTickMode (Variables|/Script/Engine.SkinnedMeshComponent|GetVisibilityBasedAnimTickOption _mesh))
  (Variables|/Script/Engine.SkinnedMeshComponent|SetVisibilityBasedAnimTickOption _mesh "AlwaysTickPoseAndRefreshBones")
  (Variables|ECAnimation|SetEC_PreMeshReplicated (Variables|/Script/Engine.ActorComponent|GetbReplicates _mesh))
  (Class|ActorComponent|SetIsReplicated _mesh false)
  (Variables|ECAnimation|SetEC_PoseReady false)
  (Variables|ECAnimation|SetEC_PoseBlend 0.0)
  (if (Ability|HasAuthority)
    (Variables|Default|SetEC_PoseFrame (Transformation|GetWorldTransform _mesh))
    (else
      (Variables|Default|SetEC_PoseFrame (.RecoveryTransform (Utilities|Struct|BreakST_EC_RagdollNetState (Variables|Default|GetEC_NetRagdollState))))
      (Physics|SetSimulatePhysics _mesh false)
      (Class|SkeletalMeshComponent|SetPhysicsBlendWeight _mesh 0.0)
      (Collision|SetCollisionEnabled _mesh "NoCollision")
      (Transformation|SetWorldTransform _mesh (Variables|Default|GetEC_PoseFrame) false true))))

(fn ECAdvancePoseBlend
  (if (Variables|ECAnimation|GetEC_PoseReady)
    (Variables|ECAnimation|SetEC_PoseBlend (Math|Float|Clamp(Float) (+ (Variables|ECAnimation|GetEC_PoseBlend) (/ (Utilities|Time|GetWorldDeltaSeconds) 0.1))))))